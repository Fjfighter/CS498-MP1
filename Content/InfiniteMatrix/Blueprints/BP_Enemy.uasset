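; BP_Enemy is an enemy that destroys itself when its Enemy component overlaps the player or a projectile.
; Touching the player calls ProcessHit on BP_Player, while touching a BP_Projectile adds one point through the player pawn's UpdateScore.
; It identifies what it touched by name strings: the object's display name for the player, the class display name for projectiles.
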(event `self.ReceiveBeginPlay`)

(event `self.Enemy.OnComponentBeginOverlap`
  (params (OverlappedComponent :type "PrimitiveComponent Object Reference") (OtherActor :type "Actor Object Reference") (OtherComp :type "PrimitiveComponent Object Reference") (OtherBodyIndex :type Integer) (bFromSweep :type Boolean) (SweepResult :type "HitResult Structure (by ref)"))
  (if (`KismetStringLibrary.EqualEqual_StrStr` (`KismetSystemLibrary.GetDisplayName` OtherActor) "BP_Player")
    (bind _asbp_player (cast `/Game/InfiniteMatrix/Blueprints/BP_Player` OtherActor))
    (`/Game/InfiniteMatrix/Blueprints/BP_Player.ProcessHit` _asbp_player)
    (`self.K2_DestroyActor`)
    (elif (`KismetStringLibrary.EqualEqual_StrStr` (`KismetSystemLibrary.GetClassDisplayName` (`GameplayStatics.GetObjectClass` OtherActor)) "BP_Projectile_C")
      (bind _asbp_player_2 (cast `/Game/InfiniteMatrix/Blueprints/BP_Player` (`GameplayStatics.GetPlayerPawn` 0)))
      (`/Game/InfiniteMatrix/Blueprints/BP_Player.UpdateScore` _asbp_player_2 1 true)
      (`self.K2_DestroyActor`))))

(fn `UserConstructionScript`)