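; BP_Projectile is a projectile actor that flies along the world X axis and destroys itself when it overlaps other actors.
; Tick offsets it by a delta-time-scaled speed, then raises that speed by a fixed amount each frame, so acceleration depends on frame rate.
; Overlaps with BP_Tunnel are ignored through a class-name comparison.
; A separate HitWall function also destroys the projectile.
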(event `self.ReceiveBeginPlay`)

(event `self.ReceiveActorBeginOverlap`
  (params (OtherActor :type "Actor Object Reference"))
  (if (not (== (`KismetStringLibrary.Conv_StringToName` (`KismetSystemLibrary.GetClassDisplayName` (`GameplayStatics.GetObjectClass` OtherActor))) "BP_Tunnel_C"))
    (`self.K2_DestroyActor`)))

(event `self.ReceiveTick`
  (params (DeltaSeconds :type "Float (single-precision)"))
  (bind _projectilespeed (`self.ProjectileSpeed`))
  (`self.K2_AddActorWorldOffset` (`KismetMathLibrary.MakeVector` (* DeltaSeconds _projectilespeed)))
  (set `self.ProjectileSpeed` (+ _projectilespeed 0.3)))

(fn `HitWall`
  (`self.K2_DestroyActor`))

(fn `UserConstructionScript`)